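; Base ant Blueprint for a grid-based movable character that occupies an ant slot on the grid and reports its death to the movable manager.
; Move advances one path cell per call, updating occupancy, facing and teleporting to the cell, then interacting with it.
; If the next cell is blocked, it recalculates with that cell forbidden, falling back to normal pathing.
; An invalid target triggers FindNewTarget, currently a placeholder.
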(event EventBeginPlay
  (bind _current (Variables|Default|GetCurrent))
  (bind (_x _y) (Utilities|Struct|BreakGridCell _current))
  (|CallParentFunction)
  (Class|GridManager|OccupyCellatIndex (Variables|Default|GetGridReference) _x _y "Ant"))

(event Collision|EventActorBeginOverlap
  (params (OtherActor :type Actor%20Object%20Reference))
  (|CallParentFunction OtherActor) ; This node is disabled and will not be called.\nDrag off pins to build functionality.
)

(event EventTick
  (params (DeltaSeconds :type Float%20%28single-precision%29))
  (|CallParentFunction DeltaSeconds))

(fn ConstructionScript
  (|CallParentFunction))

(fn Move
  (bind _path (Variables|Default|GetPath))
  (bind _gridreference (Variables|Default|GetGridReference))
  (bind _target (Variables|Default|GetTarget))
  (bind (_x _y) (Utilities|Struct|BreakGridCell _target))
  (bind _output (Utilities|Array|Get(acopy) _path))
  (bind (_x_2 _y_2) (Utilities|Struct|BreakGridCell _output))
  (bind (_x_3 _y_3) (Utilities|Struct|BreakGridCell _output))
  (if (Utilities|IsValid (Utilities|ToObject(Interface) (Variables|Default|GetTargetActor))) ; Check if target is still valid
    (if (and (== (.X (Utilities|Struct|BreakGridCell (Variables|Default|GetCurrent))) _x) (== (.Y (Utilities|Struct|BreakGridCell (Variables|Default|GetCurrent))) _y)) :!label _label ; Check if we are already at target
      (return (.X (Utilities|Struct|BreakGridCell (Variables|Default|GetCurrent))) (.Y (Utilities|Struct|BreakGridCell (Variables|Default|GetCurrent))))
      (elif (> (Utilities|Array|Length (Variables|Default|GetPath)) 0)
        (bind _returnvalue (Class|GridManager|CanActorbePlacedatIndex _gridreference _x_3 _y_3 "Ant")) ; Check if the cell is currently occupied by another ant
        (if _returnvalue
          ;[0.15 0.15 0.15 0.5] Take the first element from path and move there
          (Class|GridManager|UnoccupyCellatIndex _gridreference (.X (Utilities|Struct|BreakGridCell (Variables|Default|GetCurrent))) (.Y (Utilities|Struct|BreakGridCell (Variables|Default|GetCurrent))) "Ant" :!label _label_2) ; Walk OFF the current cell
          ;[0.15 0.15 0.15 0.5] rotate to look in the direction it will move
          (Transformation|SetActorRotation (Math|Rotator|FindLookatRotation (Math|Vector|MakeVector (Math|Conversions|ToFloat(Integer) (.X (Utilities|Struct|BreakGridCell (Variables|Default|GetCurrent)))) (Math|Conversions|ToFloat(Integer) (.Y (Utilities|Struct|BreakGridCell (Variables|Default|GetCurrent)))) 0.0) (Math|Vector|MakeVector (Math|Conversions|ToFloat(Integer) _x_2) (Math|Conversions|ToFloat(Integer) _y_2) 0.0)))
          (bind _output_get (Variables|Default|SetCurrent _output))
          (Class|GridManager|OccupyCellatIndex _gridreference (.X (Utilities|Struct|BreakGridCell _output_get)) (.Y (Utilities|Struct|BreakGridCell _output_get)) "Ant" self) ; Walk into the new cell
          (Transformation|SetActorLocation (Class|GridManager|GetWorldLocationOfGrid _gridreference (.X (Utilities|Struct|BreakGridCell _output_get)) (.Y (Utilities|Struct|BreakGridCell _output_get))) false false) ; Move there physically
          (CallFunction|InteractwithGridCell)
          (Utilities|Array|RemoveIndex _path)
          (return (.X (Utilities|Struct|BreakGridCell _output_get)) (.Y (Utilities|Struct|BreakGridCell _output_get)))
          (else
            (Development|PrintString "Target Occupied... Recalculating")
            (CallFunction|RecalculatePathingwithForbidden _output) ; I HAVE NO IDEA IF THE NODES CAN CONNECT LIKE THIS
            ;[0.15 0.15 0.15 0.5] Check if there is a path that does not require walking through that ant
            (if (> (Utilities|Array|Length (Variables|Default|GetPath)) 0)
              (goto _label_2)
              (else
                (CallFunction|RecalculatePathing) ; Reset back to normal path (can be optimised if there are performance issues)
              ))))
        (else
          ;[0.15 0.15 0.15 0.5] If no path, but not at target, reclaculate but do not move
          (CallFunction|RecalculatePathing))))
    (else
      (bind _new_target (CallFunction|FindNewTarget))
      (if (Utilities|IsValid (Utilities|ToObject(Interface) _new_target))
        (goto _label)))))

(fn TakeDamage
  (|CallParentFunction))

(fn Die
  (Default|EventKillAnt (Variables|Default|GetBPC_MovableManager) self)
  (|CallParentFunction))

(fn SetNewTarget
  (params (NewParam :type Placeable%20Interface))
  (|CallParentFunction NewParam))

(fn FindNewTarget
  ;[0.15 0.15 0.15 0.5] Null for now but ideally they should path to the nearest interactible?
  (CallFunction|SetNewTarget)
  (return 0))