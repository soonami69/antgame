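; Grid-based enemy that occupies its cell on spawn and hunts the nearest ant, found through the movable manager.
; Each Move steps along its path, updating cell occupancy, rotation and location and calling GetTrappedByGridCell.
; Reaching the target, or finding it in the blocked next cell, damages the ant and retargets as needed.
; Other blockers trigger a repath with that cell forbidden, falling back to the normal path if none exists.
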(event EventBeginPlay
  (bind _current (Variables|Default|GetCurrent))
  (bind (_x _y) (Utilities|Struct|BreakGridCell _current))
  (|CallParentFunction)
  (Class|GridManager|OccupyCellatIndex (Variables|Default|GetGridReference) _x _y "Enemy"))

(event Collision|EventActorBeginOverlap
  (params (OtherActor :type Actor%20Object%20Reference))
  (|CallParentFunction OtherActor) ; This node is disabled and will not be called.\nDrag off pins to build functionality.
)

(event EventTick
  (params (DeltaSeconds :type Float%20%28single-precision%29))
  (|CallParentFunction DeltaSeconds) ; This node is disabled and will not be called.\nDrag off pins to build functionality.
)

(fn ConstructionScript
  (|CallParentFunction))

(fn SetNewTarget
  (params (NewParam :type Placeable%20Interface))
  (bind _returnvalue (Class|Placeable|GetCurrentGrid))
  (bind _bpc_movablemanager (Variables|Default|GetBPC_MovableManager))
  (bind (_x _y) (Utilities|Struct|BreakGridCell _returnvalue))
  (if (Utilities|IsValid _bpc_movablemanager)
    (bind _ant (Default|GetAntNearesttoIndex _bpc_movablemanager _x _y))
    (if (Utilities|IsValid _ant)
      (Development|PrintString (Utilities|String|Append (Utilities|String|MakeLiteralString "Ant at: ") (Utilities|String|ToString(Integer) (.X (Utilities|Struct|BreakGridCell (Class|Placeable|GetCurrentGrid _ant)))) "," (Utilities|String|ToString(Integer) (.Y (Utilities|Struct|BreakGridCell (Class|Placeable|GetCurrentGrid _ant))))))
      (|CallParentFunction _ant)
      (else
        (Development|PrintString "No target found")))
    (else
      (Development|PrintString "No movable manager?"))))

(fn Move
  (bind _target (Variables|Default|GetTarget))
  (bind _current (Variables|Default|GetCurrent))
  (bind _target_2 (Variables|Default|GetTarget))
  (bind _current_2 (Variables|Default|GetCurrent))
  (bind _targetactor (Variables|Default|GetTargetActor))
  (bind (_x _y) (Utilities|Struct|BreakGridCell _current))
  (bind (_x_2 _y_2) (Utilities|Struct|BreakGridCell _target))
  (bind (_x_3 _y_3) (Utilities|Struct|BreakGridCell _target_2))
  (bind (_x_4 _y_4) (Utilities|Struct|BreakGridCell _current_2))
  (Utilities|IsValid (Utilities|ToObject(Interface) (Variables|Default|GetTargetActor))
    (:Is%20Valid
      (if (and (== _x _x_3) (== _y _y_3)) ; Check if we are already at target
        (bind _asbp_basic_ant (Utilities|Casting|CastToBP_Basic_Ant (Variables|Default|GetTargetActor)))
        (Default|TakeDamage _asbp_basic_ant)
        (CallFunction|SetNewTarget)
        (CallFunction|RecalculatePathing)
        (return _x_4 _y_4)
        (elif (> (Utilities|Array|Length (Variables|Default|GetPath)) 0)
          (bind _returnvalue (Class|GridManager|CanActorbePlacedatIndex (Variables|Default|GetGridReference) (.X (Utilities|Struct|BreakGridCell (stale _path_0_))) (.Y (Utilities|Struct|BreakGridCell (stale _path_0_))) "Enemy")) ; Check if the cell is currently occupied by another ant
          (if _returnvalue
            (bind (_path_0_ _new_x _new_y) (|Move,RotatenandOccupy/UnoccupyCells))
            (return _new_x _new_y)
            (else
              (Development|PrintString "Cell is already occupied by something else!")
              (if (and (== (.X (Utilities|Struct|BreakGridCell _path_0_)) _x_2) (== (.Y (Utilities|Struct|BreakGridCell _path_0_)) _y_2)) ; Check if it is the enemy in front of us
                (Development|PrintString "Enemy in front!")
                (bind _asbp_basic_ant_2 (Utilities|Casting|CastToBP_Basic_Ant _targetactor)
                  (:then
                    (Default|TakeDamage _asbp_basic_ant_2)
                    (Utilities|IsValid (Utilities|ToObject(Interface) _targetactor) ; Check if ant is dead
                      (:Is%20Valid
                        _)
                      (:Is%20Not%20Valid
                        (bind (_output _outputpin _outputpin2) (|Move,RotatenandOccupy/UnoccupyCells_2))
                        (CallFunction|SetNewTarget) ; If dead, set a new target and move to target square
                        (return _outputpin _outputpin2))))
                  (:CastFailed
                    (CallFunction|SetNewTarget)))
                (CallFunction|RecalculatePathing)
                (return _x_4 _y_4)
                (else
                  (Development|PrintString "Target Occupied... Recalculating")
                  (CallFunction|RecalculatePathingwithForbidden _path_0_)
                  ;[0.15 0.15 0.15 0.5] Check if there is a path that does not require walking through that ant
                  (if (not (> (Utilities|Array|Length (Variables|Default|GetPath)) 0))
                    (CallFunction|RecalculatePathing) ; Reset back to normal path (can be optimised if there are performance issues)
                  )))))
          (else
            ;[0.15 0.15 0.15 0.5] If no path, but not at target, reclaculate but do not move
            (CallFunction|RecalculatePathing)))))
    (:Is%20Not%20Valid
      (CallFunction|SetNewTarget))))