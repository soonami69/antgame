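; Temporary speed buff component that raises the MoveSpeed of its Basic_Mover owner and swaps the mesh material on ants and enemies.
; On BeginPlay it saves the original speed and material before applying the buff, or destroys itself if the owner is not a Basic_Mover.
; Tick decrements a frame-based Timer; at zero, HandleCleanup restores the saved values and removes the component.
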(event EventBeginPlay
  (bind _new_material (Variables|Default|GetNew%20Material))
  (Development|PrintString "Hello")
  (bind _asbasic_mover (Utilities|Casting|CastToBasic_Mover (Components|GetOwner))
    (:then
      (bind _asbp_basic_ant (Utilities|Casting|CastToBP_Basic_Ant _asbasic_mover)
        (:then
          (Variables|Default|SetOriginal%20Material (Rendering|Material|GetMaterial (Variables|/Game/Characters/Movable/BP_Basic_Ant.BP_Basic_Ant_C|GetStaticMesh _asbp_basic_ant) 0))
          (Rendering|Material|SetMaterial (Variables|/Game/Characters/Movable/BP_Basic_Ant.BP_Basic_Ant_C|GetStaticMesh _asbp_basic_ant) 0 _new_material))
        (:CastFailed
          (bind _asbp_basic_enemy (Utilities|Casting|CastToBP_Basic_Enemy _asbasic_mover)
            (:then
              (Variables|Default|SetOriginal%20Material (Rendering|Material|GetMaterial (Variables|/Game/Characters/Movable/BP_Basic_Enemy.BP_Basic_Enemy_C|GetStaticMesh _asbp_basic_enemy) 0))
              (Rendering|Material|SetMaterial (Variables|/Game/Characters/Movable/BP_Basic_Enemy.BP_Basic_Enemy_C|GetStaticMesh _asbp_basic_enemy) 0 _new_material))
            (:CastFailed
              _))))
      (bind _output_get (Variables|Default|SetInitial%20Speed (Variables|/Game/Characters/Movable/BP_Basic_Ant.BP_Basic_Ant_C|GetMove%20Speed _asbasic_mover)))
      (Variables|/Game/Characters/Movable/BP_Basic_Ant.BP_Basic_Ant_C|SetMove%20Speed _asbasic_mover (+ _output_get 1)))
    (:CastFailed
      (Development|PrintString "Attach failed!")
      (Components|DestroyComponent))))

(event EventTick
  (if (== (Variables|Default|GetTimer) 0)
    (|HandleCleanup (Components|GetOwner))
    (else
      (Variables|Default|SetTimer (- (Variables|Default|GetTimer) 1)))))