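; BP_SoundManager is a sound manager that plays background music and random ant sound effects as non-spatial 2D audio.
; On BeginPlay it spawns the music cue and keeps it in BGMPlayer, unless that player is already valid.
; The ProgressTick event plays a random ant sound at fixed volume and pitch, but only while EnableTickSound is false.
; An older Audio component music path is left unconnected.
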(event EventBeginPlay
  (Utilities|IsValid (Variables|Default|GetBGM%20Player)
    (:Is%20Not%20Valid
      (bind _returnvalue (Audio|SpawnSound2D (Variables|Default|GetBGM%20SoundCue) 1.0 1.0 0.0 0 true))
      (Variables|Default|SetBGM%20Player _returnvalue))))

(event Collision|EventActorBeginOverlap
  (params (OtherActor :type Actor%20Object%20Reference)))

(event EventTick
  (params (DeltaSeconds :type Float%20%28single-precision%29)))

(event EventProgressTick
  (if (not (Variables|Default|GetEnableTickSound))
    (Audio|PlaySound2D (.OutItem (Utilities|Array|Random (Variables|Default|GetAntSounds))) 0.9 1.2 0.0 0 0)))

(fn ConstructionScript)